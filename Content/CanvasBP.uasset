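; Paintable canvas actor that shows a runtime render target on its static mesh and accepts brush stamps.
; Clear, run at BeginPlay, creates a small black render target, binds it to a dynamic CanvasMat on the mesh, and replaces BrushMat with a dynamic instance.
; DrawOnCanvas sets the brush texture on that instance and draws it into the target, centred on a normalised location at the given pixel size.
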(event `self.ReceiveBeginPlay`
  (`self.Clear`))

(event `Clear`
  (bind _returnvalue (`KismetRenderingLibrary.CreateRenderTarget2D` 32 32 "RTF_RGBA8"))
  (bind _output_get (set `self.Render` _returnvalue))
  (`KismetRenderingLibrary.ClearRenderTarget2D` _output_get)
  (bind _returnvalue_2 (`KismetMaterialLibrary.CreateDynamicMaterialInstance` "/Game/CanvasMat.CanvasMat"))
  (`MaterialInstanceDynamic.SetTextureParameterValue` _returnvalue_2 "Target" (`self.Render`))
  (`PrimitiveComponent.SetMaterial` (`self.StaticMesh`) 0 _returnvalue_2)
  (bind _returnvalue_3 (`KismetMaterialLibrary.CreateDynamicMaterialInstance` "/Game/BrushMat.BrushMat"))
  (set `self.BrushMat` _returnvalue_3))

(fn `DrawOnCanvas`
  (params (`Brush Texture` :type "Texture2D Object Reference") (Size :type "Float (double-precision)") (Location :type "Vector2D Structure"))
  (`|ExecutionSequence`
    (:`then_0`
      (`MaterialInstanceDynamic.SetTextureParameterValue` (`self.BrushMat`) "Brush" `Brush Texture`))
    (:`then_1`
      (bind (_canvas _size _context) (`KismetRenderingLibrary.BeginDrawCanvasToRenderTarget` (`self.Render`)))
      (`Canvas.K2_DrawMaterial` _canvas (`self.BrushMat`) (- (* _size Location) (/ Size 2.0)) (`KismetMathLibrary.MakeVector2D` Size Size) (0.0 0.0) (1.0 1.0) 0.0 (0.5 0.5))
      (`KismetRenderingLibrary.EndDrawCanvasToRenderTarget` _context))))

(fn `UserConstructionScript`)