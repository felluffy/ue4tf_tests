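; Player pawn Blueprint with basic walk and look controls plus two test key actions.
; Axis inputs move along control-yaw forward and right vectors, keeping movement planar, and feed controller pitch and yaw.
; Left click draws a persistent debug line trace from the eye point along actor forward, without using the hit.
; The 6 key sends a text request with a random id query through HTTP.
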(event `Key|Six`
  (params (Key :type "Key Structure"))
  (:`Pressed`
    (`HTTPComponent.SendTextRequest` (`self.HTTP`) (`KismetStringLibrary.Concat_StrStr` "?id=" (`KismetStringLibrary.Conv_IntToString` (`KismetMathLibrary.RandomInteger` 31431))) false)))

(event `InputAxis|Input Axis Move Forward`
  (params (AxisValue :type "Float (single-precision)"))
  (`self.AddMovementInput` (`KismetMathLibrary.GetForwardVector` (`KismetMathLibrary.MakeRotator` 0.0 0.0 (.yaw (`self.GetControlRotation`)))) AxisValue))

(event `InputAxis|Input Axis Move Right`
  (params (AxisValue :type "Float (single-precision)"))
  (`self.AddMovementInput` (`KismetMathLibrary.GetRightVector` (`KismetMathLibrary.MakeRotator` 0.0 0.0 (.yaw (`self.GetControlRotation`)))) AxisValue))

(event `InputAxis|Input Rotate Up`
  (params (AxisValue :type "Float (single-precision)"))
  (`self.AddControllerPitchInput` AxisValue))

(event `InputAxis|Input Rotate Right`
  (params (AxisValue :type "Float (single-precision)"))
  (`self.AddControllerYawInput` AxisValue))

(event `Key|LeftMouseButton`
  (params (Key :type "Key Structure"))
  (bind _outlocation (`self.GetActorEyesViewPoint`))
  (:`Pressed`
    (`KismetSystemLibrary.LineTraceSingle` :`Start` _outlocation :`End` (+ _outlocation (* (`self.GetActorForwardVector`) 200.0)) :`TraceChannel` "TraceTypeQuery1" :`bTraceComplex` true :`DrawDebugType` "Persistent")))

(fn `UserConstructionScript`)